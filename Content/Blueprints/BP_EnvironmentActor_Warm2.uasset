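; BP_EnvironmentActor_Warm2 is an environment actor that drives a material color and scalar value, starting black and turning red.
; Tick runs through a three-second Delay, so the change to red reapplies repeatedly rather than firing once.
; Custom events switch the color to red or blue or set a high or low scalar.
; These events and BeginPlay all feed UpdateMaterialParameters, which is defined outside these graphs.
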(event `self.ReceiveTick`
  (params (DeltaSeconds :type "Float (single-precision)"))
  (`KismetSystemLibrary.Delay` 3.0)
  (`self.ChangeMatColorToRed`))

(event `IncMatScalarValue`
  (set `self.MaterialScalarValue` 300.0)
  (`self.UpdateMaterialParameters` :!label _label))

(event `DecMatScalarValue`
  (set `self.MaterialScalarValue` 10.0)
  (goto _label))

(event `self.ReceiveBeginPlay`
  (set `self.MaterialColor` (struct))
  (goto _label))

(event `ChangeMatColorToBlue`
  (set `self.MaterialColor` (struct :`B` 1.0 :`A` 1.0))
  (goto _label))

(event `ChangeMatColorToRed`
  (set `self.MaterialColor` (struct :`R` 1.0 :`A` 1.0))
  (goto _label))

(fn `UserConstructionScript`)