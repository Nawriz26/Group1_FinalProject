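; Environment actor that periodically alternates its material between two looks, blue with a high scalar value and red with a zero scalar.
; Tick runs through a three-second Delay, which acts as a repeating timer driving two FlipFlops, one for the scalar and one for the color.
; Each branch fires a custom event that sets MaterialScalarValue or MaterialColor, then calls UpdateMaterialParameters, which is not defined in this graph.
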(event `IncMatScalarValue`
  (set `self.MaterialScalarValue` 500.0)
  (`self.UpdateMaterialParameters` :!label _label))

(event `DecMatScalarValue`
  (set `self.MaterialScalarValue` 0.0)
  (goto _label))

(event `ChangeMatColorToBlue`
  (set `self.MaterialColor` (struct :`R` 0.069565 :`G` 0.191304 :`B` 1.0 :`A` 1.0))
  (goto _label))

(event `ChangeMatColorToRed`
  (set `self.MaterialColor` (struct :`R` 1.0 :`G` 0.069565 :`B` 0.069565 :`A` 1.0))
  (goto _label))

(event `self.ReceiveBeginPlay`)

(event `self.ReceiveTick`
  (params (DeltaSeconds :type "Float (single-precision)"))
  (`KismetSystemLibrary.Delay` 3.0)
  (`/Engine/EditorBlueprintResources/StandardMacros.FlipFlop`
    (:`A`
      (`self.IncMatScalarValue`))
    (:`B`
      (`self.DecMatScalarValue`)))
  (`/Engine/EditorBlueprintResources/StandardMacros.FlipFlop`
    (:`A`
      (`self.ChangeMatColorToBlue`))
    (:`B`
      (`self.ChangeMatColorToRed`))))

(fn `UserConstructionScript`)